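; Spirit1 is a grabbable bottle, held by motion controller, that pours a liquid ingredient into containers.
; Each tick, it compares the bottle's up vector to a tilt threshold to toggle a Niagara pour stream tinted with the liquid colour.
; While pouring, a downward trace from the pour point sends ingredient, colour and time-scaled amount to any actor hit that implements BPI_Container.
; Grab and Release only track the holding controller reference.
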(event `/Game/Interfaces/Grab.Grab`
  (params (MotionController :type "MotionControllerComponent Object Reference"))
  (set `self.Motion Controller` MotionController))

(event `/Game/Interfaces/Grab.Release`
  (params (MotionController :type "MotionControllerComponent Object Reference"))
  (if (== MotionController (`self.Motion Controller`))
    (set `self.Motion Controller` null)))

(event `self.ReceiveBeginPlay`
  (`NiagaraComponent.SetNiagaraVariableLinearColor` (`self.PourStream`) "User.LiquidColour" (`self.LiquidColour`)))

(event `self.ReceiveTick`
  (params (DeltaSeconds :type "Float (single-precision)"))
  (bind _returnvalue (`SceneComponent.K2_GetComponentLocation` (`self.PourPoint`)))
  (if (< (`KismetMathLibrary.Dot_VectorVector` (`SceneComponent.GetUpVector` (`self.Bottle`)) (0.0 0.0 1.0)) (`self.PourThreshold`))
    (if (not (`self.bIsPouring`))
      (`ActorComponent.Activate` (`self.PourStream`) true)
      (set `self.bIsPouring` true))
    (bind _outhit (`KismetSystemLibrary.LineTraceSingle` _returnvalue (- _returnvalue (`KismetMathLibrary.MakeVector` 0.0 0.0 (`self.TraceLength`))) "TraceTypeQuery1" false (`|MakeArray` self :!type "Actor Object Reference") "ForOneFrame"))
    (bind (_bblockinghit _binitialoverlap _time _distance _location _impactpoint _normal _impactnormal _physmat _hitactor) (`GameplayStatics.BreakHitResult` _outhit))
    (if (`KismetSystemLibrary.DoesImplementInterface` _hitactor "/Game/Blueprints/BPI_Container.BPI_Container_C")
      (message `/Game/Blueprints/BPI_Container.ReceiveLiquid` _hitactor (`self.Ingredient`) (* (`self.PourRate`) DeltaSeconds) (`self.LiquidColour`)))
    (elif (`self.bIsPouring`)
      (`ActorComponent.Deactivate` (`self.PourStream`))
      (set `self.bIsPouring` false))))

(fn `UserConstructionScript`)