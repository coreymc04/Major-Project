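; Stein is a motion-controller grabbable container that tracks how full it is.
; Grab stores the holding controller and Release clears it only for that same controller, with no attachment or physics logic here.
; Fill adds the given amount while the level is below 100, without clamping the result, and prints the new level.
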(event `/Game/Interfaces/Grab.Grab`
  (params (MotionController :type "MotionControllerComponent Object Reference"))
  (set `self.Motion Controller` MotionController))

(event `/Game/Interfaces/Grab.Release`
  (params (MotionController :type "MotionControllerComponent Object Reference"))
  (if (== MotionController (`self.Motion Controller`))
    (set `self.Motion Controller` null)))

(event `/Game/Blueprints/bpi_drinkInteractions.Fill`
  (params (FillAmount :type "Float (double-precision)"))
  (if (< (`self.FillLevel`) 100.0)
    (bind _output_get (set `self.FillLevel` (+ (`self.FillLevel`) FillAmount)))
    (`KismetSystemLibrary.PrintString` (`KismetStringLibrary.Conv_DoubleToString` _output_get))))

(fn `UserConstructionScript`)