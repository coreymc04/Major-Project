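; Grabbable drink shaker for motion controllers that collects poured ingredients and shows the mixed liquid inside.
; Grab and Release track the holding controller.
; Until full, each Liquid event totals amounts per ingredient, listing an ingredient in Contents once it reaches AddThreshold.
; It also raises the fill level, scales the liquid mesh's height through LiquidRoot, and blends colour by volume share into a dynamic material.
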(event `self.Grab`
  (params (MotionController :type "MotionControllerComponent Object Reference"))
  (set `self.Motion Controller` MotionController))

(event `self.Release`
  (params (MotionController :type "MotionControllerComponent Object Reference"))
  (if (== MotionController (`self.Motion Controller`))
    (set `self.Motion Controller` null)))

(event `self.ReceiveBeginPlay`
  (bind _returnvalue (`PrimitiveComponent.CreateDynamicMaterialInstance` (`self.LiquidMesh`) 0 "/Game/Blueprints/M_Liquid.M_Liquid" "None"))
  (set `self.LiquidMID` _returnvalue)
  (`SceneComponent.SetRelativeScale3D` (`self.LiquidRoot`) (1.0 1.0 0.01))
  (`SceneComponent.SetVisibility` (`self.LiquidMesh`) false false))

(event `self.ReceiveLiquid`
  (params (Ingredient :type "/Game/Blueprints/E_Ingredient Enum" :default "NewEnumerator0") (Amount :type "Float (double-precision)") (Colour :type "LinearColor Structure"))
  (bind _returnvalue (+ (`BlueprintMapLibrary.Map_Find` (`self.PourTimes`) Ingredient) Amount))
  (if (not (>= (`self.FillLevel`) 0.275))
    (`BlueprintMapLibrary.Map_Add` (`self.PourTimes`) Ingredient _returnvalue)
    (if (>= _returnvalue (`self.AddThreshold`))
      (`KismetArrayLibrary.Array_AddUnique` (`self.Contents`) Ingredient))
    (set `self.FillLevel` (`KismetMathLibrary.FClamp` (+ (/ Amount (`self.MaxVolume`)) (`self.FillLevel`)) 0.0 0.275))
    (set `self.CurrentColour` (`KismetMathLibrary.LinearColorLerp` (`self.CurrentColour`) Colour (/ Amount (* (`self.FillLevel`) (`self.MaxVolume`)))))
    (`SceneComponent.SetVisibility` (`self.LiquidMesh`) true false)
    (`SceneComponent.SetRelativeScale3D` (`self.LiquidRoot`) (`KismetMathLibrary.MakeVector` 4.435 7.6075 (`KismetMathLibrary.FMax` (`self.FillLevel`) 0.01)))
    (`MaterialInstanceDynamic.SetVectorParameterValue` (`self.LiquidMID`) "LiquidColour" (`self.CurrentColour`))
    (`KismetSystemLibrary.PrintString` (`KismetStringLibrary.Conv_DoubleToString` (`self.FillLevel`)))))

(fn `UserConstructionScript`)